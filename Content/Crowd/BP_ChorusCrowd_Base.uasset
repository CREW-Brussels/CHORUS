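; Base Blueprint for CHORUS crowd actors, hidden in game at BeginPlay, that drives looped playback between recorded cues through the CHORUS subsystem.
; StartRecording stores the start cue, and EndRecording stores the end cue, resets speed and starts a palindrome loop via ControlPlayer.
; SetPlaySpeed forwards speed changes to the subsystem.
; GetSkeletonLocation is a stub for specialized children to override, printing a warning and returning zero.
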(event Custom|Start%20Recording
  (params (Cue :type Chorus%20Cue%20Point%20Structure))
  (Variables|Default|SetStart%20Cue Cue))

(event Custom|End%20Recording
  (params (Cue :type Chorus%20Cue%20Point%20Structure))
  (Variables|Default|SetEnd%20Cue Cue)
  (Variables|Default|SetPlay%20Speed 1.0)
  (Class|CHORUSSubsystem|ControlPlayer (Subsystems|GetCHORUSSubsystem) self (Variables|Default|GetStart%20Cue) (Variables|Default|GetEnd%20Cue) (Variables|Default|GetPlay%20Speed) true true true))

(event Custom|Set%20Play%20Speed
  (params (Speed :type Float%20%28double-precision%29))
  (bind _output_get (Variables|Default|SetPlay%20Speed Speed))
  (Class|CHORUSSubsystem|SetPlayerSpeed (Subsystems|GetCHORUSSubsystem) self _output_get))

(event EventBeginPlay
  (Rendering|SetActorHiddenInGame true))

(fn ConstructionScript)

(fn GetSkeletonLocation
  (Development|PrintString "Override GetSkeletonLocation in specialized ChorusCrowd Blueprint" true true "(R=1.000000,G=0.000000,B=0.018845,A=1.000000)" 2.0 "ChorusCrowd")
  (return "0, 0, 0"))