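; Manages a pre-spawned pool of crowd actors that can be spawned, possessed, discarded and recorded one at a time.
; Spawn takes the next pool member round-robin; Discard and Possess release Current, or call FindClosest if none is held.
; FindClosest's inverted distance test only accepts very distant visible members, otherwise falling back to round-robin.
; Record toggles CHORUSSubsystem capture on Current, and releasing Current stops any active recording.
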(event Custom|Spawn
  (params (RecordOwner :type Actor%20Object%20Reference))
  (Utilities|IsValid (Variables|Default|GetCurrent)
    (:Is%20Valid
      (CallFunction|CheckRecording RecordOwner))
    (:Is%20Not%20Valid
      _))
  (bind _next (CallFunction|GetNextCrowd))
  (Variables|Default|SetCurrent _next)
  (Variables|/CHORUS/Crowd/BP_ChorusCrowd_Base.BP_ChorusCrowd_Base_C|SetPossessed (Variables|Default|GetCurrent) true)
  (Rendering|SetActorHiddenInGame (Variables|Default|GetCurrent) true)
  (Utilities|FlowControl|Delay (Variables|Default|GetFade%20Time))
  (Rendering|SetActorHiddenInGame (Variables|Default|GetCurrent) false))

(event Custom|Discard
  (params (Location :type Vector) (RecordOwner :type Actor%20Object%20Reference))
  (Utilities|IsValid (Variables|Default|GetCurrent)
    (:Is%20Valid
      (CallFunction|CheckRecording RecordOwner)
      (Rendering|SetActorHiddenInGame (Variables|Default|GetCurrent) true)
      (Variables|Default|SetCurrent 0))
    (:Is%20Not%20Valid
      (bind _closest (CallFunction|FindClosest Location))
      (Rendering|SetActorHiddenInGame _closest true))))

(event Custom|Possess
  (params (Location :type Vector) (RecordOwner :type Actor%20Object%20Reference))
  (Utilities|IsValid (Variables|Default|GetCurrent)
    (:Is%20Valid
      (CallFunction|CheckRecording RecordOwner)
      (Variables|Default|SetCurrent 0))
    (:Is%20Not%20Valid
      (bind _closest (CallFunction|FindClosest Location))
      (bind _output_get (Variables|Default|SetCurrent _closest))
      (Variables|/CHORUS/Crowd/BP_ChorusCrowd_Base.BP_ChorusCrowd_Base_C|SetPossessed _output_get true)
      (if (Variables|/Script/Engine.Actor|GetbHidden (Variables|Default|GetCurrent))
        (Utilities|FlowControl|Delay (Variables|Default|GetFade%20Time))
        (Rendering|SetActorHiddenInGame (Variables|Default|GetCurrent) true)))))

(event Custom|Record
  (params (RecordOwner :type Actor%20Object%20Reference))
  (Utilities|IsValid (Variables|Default|GetCurrent)
    (:Is%20Valid
      (if (Variables|Default|GetRecording)
        (CallFunction|StopRecording RecordOwner)
        (else
          (Variables|Default|SetRecording true)
          (bind _cuepoint (Class|CHORUSSubsystem|StartRecording (Subsystems|GetCHORUSSubsystem) RecordOwner))
          (Default|StartRecording (Variables|Default|GetCurrent) _cuepoint))))))

(event EventBeginPlay
  (for _index (range 1 (Variables|Default|GetPool%20Size))
    (bind _returnvalue (Game|SpawnActorfromClass (Variables|Default|GetCrowd%20Class) (Math|Transform|MakeTransform "0, 0, 0" "0, 0, 0" "1.000000,1.000000,1.000000") "Undefined" "MultiplyWithRoot" 0 0))
    (Utilities|Array|Add (Variables|Default|GetCrowd) _returnvalue)))

(event Collision|EventActorBeginOverlap
  (params (OtherActor :type Actor%20Object%20Reference)))

(event EventTick
  (params (DeltaSeconds :type Float%20%28single-precision%29)))

(fn ConstructionScript)

(fn StopRecording
  (params (RecordOwner :type Actor%20Object%20Reference))
  (Variables|Default|SetRecording false)
  (bind _cuepoint (Class|CHORUSSubsystem|StopRecording (Subsystems|GetCHORUSSubsystem) RecordOwner))
  (Default|EndRecording (Variables|Default|GetCurrent) _cuepoint))

(fn FindClosest
  (params (Location :type Vector))
  (LocalVariables|SetClosest%20Distance 1e+08)
  (LocalVariables|SetClosest%20Ref 0)
  (for _array_element (Variables|Default|GetCrowd)
    (if (not (Variables|/Script/Engine.Actor|GetbHidden _array_element))
      (bind _location (Default|GetSkeletonLocation _array_element))
      (if (< (LocalVariables|GetClosest%20Distance) (Class|KismetMathLibrary|VectorDistanceSquared _location Location))
        (LocalVariables|SetClosest%20Distance (Class|KismetMathLibrary|VectorDistanceSquared _location Location))
        (LocalVariables|SetClosest%20Ref _array_element))))
  (Utilities|IsValid (LocalVariables|GetClosest%20Ref)
    (:Is%20Valid
      (return (LocalVariables|GetClosest%20Ref)))
    (:Is%20Not%20Valid
      (bind _next (CallFunction|GetNextCrowd))
      (return _next))))

(fn GetNextCrowd
  (LocalVariables|SetRef (Utilities|Array|Get(acopy) (Variables|Default|GetCrowd) (Variables|Default|GetIndex)))
  (Variables|Default|SetIndex (Math|Integer|%(Integer) (+ (Variables|Default|GetIndex) 1) (Utilities|Array|Length (Variables|Default|GetCrowd))))
  (return (LocalVariables|GetRef)))

(fn CheckRecording
  (params (RecordOwner :type Actor%20Object%20Reference))
  (if (Variables|Default|GetRecording)
    (CallFunction|StopRecording RecordOwner))
  (Variables|/CHORUS/Crowd/BP_ChorusCrowd_Base.BP_ChorusCrowd_Base_C|SetPossessed (Variables|Default|GetCurrent) false)
  (return))