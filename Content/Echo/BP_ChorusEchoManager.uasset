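; Manager actor that uses the CHORUS subsystem to record a target and launch staggered echo actors from that recording.
; BeginPlay pre-spawns an echo pool and binds track-end events, which call EchoEnd on the owning echo.
; Start begins recording, then a delayed self-calling Echo event cycles round-robin through the pool, launching at most PoolSize echoes per Start.
; Stop clears the echoing flag and ends the recording.
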(event Custom|On%20Track%20End
  (params (Subsystem :type CHORUS%20Subsystem%20Object%20Reference) (Owner :type Actor%20Object%20Reference) (Track :type Integer))
  (bind _asbp_chorus_echo_base (Utilities|Casting|CastToBP_ChorusEcho_Base Owner))
  (Default|EchoEnd _asbp_chorus_echo_base))

(event Custom|Echo
  (if (> (Variables|Default|GetCount) 0)
    (Math|Integer|DecrementInt (Variables|Default|GetCount)
      (:%20%20
        (Default|EchoStart (Utilities|Array|Get(acopy) (Variables|Default|GetEchoes) (Variables|Default|GetIndex)) (Variables|Default|GetEcho%20Start))
        (Variables|Default|SetIndex (Math|Integer|%(Integer) (+ (Variables|Default|GetIndex) 1) (Utilities|Array|Length (Variables|Default|GetEchoes))))
        (if (Variables|Default|GetEchoing)
          (Utilities|FlowControl|Delay (Variables|Default|GetDelay))
          (CallFunction|Echo))))))

(event Custom|Start
  (params (Target :type Actor%20Object%20Reference))
  (bind _cuepoint (Class|CHORUSSubsystem|StartRecording (Subsystems|GetCHORUSSubsystem) Target))
  (if (!= (.Track (Utilities|Struct|BreakChorusCuePoint _cuepoint)) 0)
    (Variables|Default|SetEcho%20Start _cuepoint)
    (Variables|Default|SetCount (Variables|Default|GetPool%20Size))
    (Variables|Default|SetEchoing true)
    (Utilities|FlowControl|Delay (Variables|Default|GetDelay))
    (CallFunction|Echo)))

(event Custom|Stop
  (params (Target :type Actor%20Object%20Reference))
  (Variables|Default|SetEchoing false)
  (Class|CHORUSSubsystem|StopRecording (Subsystems|GetCHORUSSubsystem) Target))

(event EventBeginPlay
  (EventDispatchers|BindEventtoOnEndOfTrack (Subsystems|GetCHORUSSubsystem) (delegate Custom|On%20Track%20End))
  (for _index (range 1 (Variables|Default|GetPool%20Size))
    (bind _returnvalue (Game|SpawnActorfromClass (Variables|Default|GetEcho%20Class) (Math|Transform|MakeTransform "0, 0, 0" "0, 0, 0" "1.000000,1.000000,1.000000") "Undefined" "MultiplyWithRoot" 0 0))
    (Utilities|Array|Add (Variables|Default|GetEchoes) _returnvalue)))

(fn ConstructionScript)